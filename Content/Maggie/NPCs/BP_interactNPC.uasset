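; BP_interactNPC is a sick NPC that the player can cure with crafted medicine.
; On overlap it prints a plea for help or a cured message, depending on IsSick, and ending the overlap clears a Person flag.
; Clicking its mesh checks MedicineCrafted on the first-person character; if true, the mesh switches to a green flower material and IsSick is cleared.
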(event `self.ReceiveActorBeginOverlap`
  (params (OtherActor :type "Actor Object Reference"))
  (if (`self.Is sick`)
    (`KismetSystemLibrary.PrintString` "I am sick. Can you help me?")
    (else
      (`KismetSystemLibrary.PrintString` "You Have cured me!"))))

(event `self.ReceiveActorEndOverlap`
  (params (OtherActor :type "Actor Object Reference"))
  (set `self.Person` false))

(event `self.NPCMeshOnlyfbx2.OnClicked`
  (params (TouchedComponent :type "PrimitiveComponent Object Reference") (ButtonPressed :type "Key Structure"))
  (bind _asbp_first_person_character (cast `/Game/FirstPerson/Blueprints/BP_FirstPersonCharacter` (`GameplayStatics.GetPlayerCharacter` 0)))
  (if (`/Game/FirstPerson/Blueprints/BP_FirstPersonCharacter.Medicine Crafted` _asbp_first_person_character)
    (`PrimitiveComponent.SetMaterial` (`self.NPCMeshOnlyfbx2`) 0 "/Game/Bonnie/Objects/Flowers/FlowerGreen.FlowerGreen")
    (set `self.Is sick` false)))

(fn `UserConstructionScript`)