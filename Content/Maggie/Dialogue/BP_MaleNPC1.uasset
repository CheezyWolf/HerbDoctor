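; BP_MaleNPC1 is a male NPC Blueprint that steps through lines of dialogue when its Talk event fires.
; Each call increments TalkIdeck and, while it is within the Dialogue array, clears the UITalk reference and passes that line to SetText.
; The chain that creates a UI_Dialogue widget, stores it in UITalk and adds it to the viewport is disconnected, so it never runs.
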(event `/Game/Maggie/Dialogue/Bp_Dialogue.Talk`
  (`/Engine/EditorBlueprintResources/StandardMacros.IncrementInt` (`self.TalkIdeck`)
    (:`  `
      (if (< (`self.TalkIdeck`) (`KismetArrayLibrary.Array_Length` (`self.Dialogue`)))
        (set `self.UITalk` null)
        (`TextBlock.SetText` (`KismetTextLibrary.Conv_StringToText` (`|GetArrayItem` (`self.Dialogue`) (`self.TalkIdeck`))))))))

(fn `UserConstructionScript`)