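; BP_InventoryComponent is an inventory component that tracks item quantities by name in an Inventory map.
; AddItem adds the amount to an existing count or creates a new entry, and GetItemCount returns the stored count.
; RemoveItem subtracts with a floor of zero and writes the result back, so depleted items stay in the map.
; The component has no active event logic.
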(fn `AddItem`
  (params (ItemName :type Name) (Amount :type Integer))
  (bind (_value _returnvalue) (`BlueprintMapLibrary.Map_Find` (`self.Inventory`) ItemName))
  (if _returnvalue
    (`BlueprintMapLibrary.Map_Add` (`self.Inventory`) ItemName (+ _value Amount))
    (else
      (`BlueprintMapLibrary.Map_Add` (`self.Inventory`) ItemName Amount))))

(fn `GetItemCount`
  (params (ItemName :type Name))
  (returns (Count :type Integer))
  (return (`BlueprintMapLibrary.Map_Find` (`self.Inventory`) ItemName)))

(fn `RemoveItem`
  (params (ItemName :type Name) (Amount :type Integer))
  (`BlueprintMapLibrary.Map_Add` (`self.Inventory`) ItemName (`KismetMathLibrary.Max` (- (`BlueprintMapLibrary.Map_Find` (`self.Inventory`) ItemName) Amount))))