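; Day manager that runs a three-day villager choice loop, pairing two villagers each day and ending with a win screen.
; StartDay loads the day's pair from DayPairings; PlayerChose notifies the saved and abandoned villagers, then advances the day or triggers the ending.
; Between days it shows a Days widget, teleports the player and briefly disables movement.
; ShowChoiceUi is empty here, and the choice-widget setup is disconnected.
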(event `self.ReceiveBeginPlay`
  (`self.StartDay`))

(event `TriggerEnding`
  (bind _returnvalue (`|CreateWidget` "/Game/Widgets/YouWin_WGT.YouWin_WGT_C"))
  (`UserWidget.AddToViewport` _returnvalue 0))

(event `ShowChoiceUi`)

(event `OnVillagerChosen_Response`
  (params (ChosenVillager :type "/Game/Beatriz/ReWork/Villagers/BP_VIllager_Base Object Reference"))
  (`self.PlayerChose(ChosenVillager)` ChosenVillager))

(event `OnDayProgressed`
  (bind _charactermovement (`Character.CharacterMovement` (stale _returnvalue_2)))
  (`CharacterMovementComponent.SetMovementMode` _charactermovement "MOVE_None" 0)
  (bind _returnvalue (`|CreateWidget` "/Game/Widgets/Days_WGT.Days_WGT_C"))
  (`UserWidget.AddToViewport` _returnvalue 0)
  (bind _returnvalue_2 (`GameplayStatics.GetActorOfClass` "/Game/FirstPerson/Blueprints/BP_FirstPersonCharacter.BP_FirstPersonCharacter_C"))
  (`self.K2_SetActorLocation` _returnvalue_2 (-440.0 150.0 92.0001) false false)
  (`KismetSystemLibrary.Delay` 3.0)
  (`CharacterMovementComponent.SetMovementMode` _charactermovement "MOVE_Walking" 0)
  (`Widget.RemoveFromParent` _returnvalue))

(fn `PlayerChose(ChosenVillager)`
  (params (ChosenVillager :type "/Game/Beatriz/ReWork/Villagers/BP_VIllager_Base Object Reference"))
  (bind _villagera (`self.VillagerA`))
  (bind _villagerb (`self.VillagerB`))
  (`KismetSystemLibrary.PrintString` "Player Chose started")
  (if (== ChosenVillager (`self.VillagerA`))
    (`/Game/Beatriz/ReWork/Villagers/BP_VIllager_Base.OnAbandoned` _villagerb)
    (`KismetSystemLibrary.PrintString` (`/Game/Beatriz/ReWork/Villagers/BP_VIllager_Base.VillagerRole` _villagerb))
    (`/Game/Beatriz/ReWork/Villagers/BP_VIllager_Base.OnSaved` (`self.VillagerA`))
    (else
      (`/Game/Beatriz/ReWork/Villagers/BP_VIllager_Base.OnAbandoned` _villagera)
      (`KismetSystemLibrary.PrintString` (`/Game/Beatriz/ReWork/Villagers/BP_VIllager_Base.VillagerRole` _villagera))
      (`/Game/Beatriz/ReWork/Villagers/BP_VIllager_Base.OnSaved` (`self.VillagerB`))))
  (bind _result (`/Engine/EditorBlueprintResources/StandardMacros.IncrementInt` (`self.CurrentDay`))
    (:`  `
      (bind _output_get (set `self.CurrentDay` _result))
      (`KismetSystemLibrary.PrintString` (`KismetStringLibrary.Conv_IntToString` (+ _output_get 1)))
      (if (== (`self.CurrentDay`) 3)
        (`self.TriggerEnding`)
        (else
          (`self.OnDayProgressed`)
          (`self.StartDay`))))))

(fn `StartDay`
  (bind (_villagera _villagerb) (break `/Game/Beatriz/ReWork/S_DayPairing` (`|GetArrayItem` (`self.DayPairings`) (`self.CurrentDay`))))
  (set `self.VillagerA` _villagera)
  (set `self.VillagerB` _villagerb)
  (`KismetSystemLibrary.PrintString` (`/Game/Beatriz/ReWork/Villagers/BP_VIllager_Base.VillagerName` _villagera))
  (`KismetSystemLibrary.PrintString` (`/Game/Beatriz/ReWork/Villagers/BP_VIllager_Base.VillagerName` _villagerb))
  (`self.ShowChoiceUI`))

(fn `UserConstructionScript`)