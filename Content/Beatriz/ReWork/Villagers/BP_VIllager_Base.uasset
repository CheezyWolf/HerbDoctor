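; Base villager actor that may be sick and can be clicked to be offered a cure.
; A sphere overlap toggles its text render and, for the player, an interact prompt; a component named "1" shows when sick.
; Clicking a sick villager checks the player's inventory for a Cure, then opens a UI-only confirmation widget.
; OnSaved records the villager and OnAbandoned destroys it; the DayManager check on Tick does nothing.
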(event `self.ReceiveBeginPlay`
  (bind __1 (`self.!1`))
  (bind _returnvalue (`|CreateWidget` "/Game/Bonnie/UIs/Npc_Interact.Npc_Interact_C"))
  (set `self.Interactprompt` _returnvalue)
  (set `PlayerController.bEnableClickEvents` true (`GameplayStatics.GetPlayerController` 0))
  (`SceneComponent.SetVisibility` (`self.TextRender`) false false)
  (bind _outactors (`GameplayStatics.GetAllActorsOfClass` "/Game/Beatriz/ReWork/BP_DayManager.BP_DayManager_C"))
  (if (`self.IsSick?`)
    (`SceneComponent.SetVisibility` __1 true true)
    (else
      (`SceneComponent.SetVisibility` __1 false true))))

(event `self.ReceiveTick`
  (params (DeltaSeconds :type "Float (single-precision)"))
  (if (== (`/Game/Beatriz/ReWork/BP_DayManager.CurrentDay` (`|GetArrayItem` (stale `self.ReceiveBeginPlay` _outactors))) 0)
    _))

(event `OnSaved`
  (`KismetSystemLibrary.PrintString` "Saved character")
  (set `self.Saved Character` self))

(event `OnAbandoned`
  (`KismetSystemLibrary.PrintString` "Abandoned character")
  (`self.K2_DestroyActor` self))

(event `self.Mesh.OnClicked`
  (params (TouchedComponent :type "PrimitiveComponent Object Reference") (ButtonPressed :type "Key Structure"))
  (if (`self.IsSick?`)
    (bind _count (`/Game/Beatriz/ReWork/BP_InventoryComponent.GetItemCount` (`self.GetComponentByClass` (`GameplayStatics.GetPlayerCharacter` 0) "/Game/Beatriz/ReWork/BP_InventoryComponent.BP_InventoryComponent_C") "Cure"))
    (`KismetSystemLibrary.PrintString` (`KismetStringLibrary.Conv_IntToString` _count))
    (if (>= _count 1)
      (`self.ShowConfirmationPopUp`))))

(event `ShowConfirmationPopUp`
  (bind _returnvalue (`|CreateWidget` "/Game/Beatriz/ReWork/WGT_ConfirmCure.WGT_ConfirmCure_C"))
  (bind _output_get (set `self.ConfirmWgt` _returnvalue))
  (`UserWidget.AddToViewport` _output_get 0)
  (`WidgetBlueprintLibrary.SetInputMode_UIOnlyEx` (`GameplayStatics.GetPlayerController` 0) null)
  (`/Game/Beatriz/ReWork/WGT_ConfirmCure.InitConfirmWidget` _output_get self))

(event `self.Sphere.OnComponentBeginOverlap`
  (params (OverlappedComponent :type "PrimitiveComponent Object Reference") (OtherActor :type "Actor Object Reference") (OtherComp :type "PrimitiveComponent Object Reference") (OtherBodyIndex :type Integer) (bFromSweep :type Boolean) (SweepResult :type "HitResult Structure (by ref)"))
  (`SceneComponent.SetVisibility` (`self.TextRender`) true false)
  (if (== OtherActor (`GameplayStatics.GetPlayerCharacter` 0))
    (`UserWidget.AddToViewport` (`self.Interactprompt`) 0)))

(event `self.Sphere.OnComponentEndOverlap`
  (params (OverlappedComponent :type "PrimitiveComponent Object Reference") (OtherActor :type "Actor Object Reference") (OtherComp :type "PrimitiveComponent Object Reference") (OtherBodyIndex :type Integer))
  (`SceneComponent.SetVisibility` (`self.TextRender`) false false)
  (if (== OtherActor (`GameplayStatics.GetPlayerCharacter` 0))
    (`Widget.RemoveFromParent` (`self.Interactprompt`))))

(fn `UserConstructionScript`)