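; BP_Villager_Leader is the villager leader, a child Blueprint that shows sickness on day two and can open a tutorial when clicked.
; Every Tick it reads CurrentDay from BP_DayManager, toggling IsSick, component "1" visibility and a looping sick or idle animation, re-issuing PlayAnimation each frame.
; Clicking the mesh while FirstClickTutorial is true opens Tutorial_WGT with UI-only input, a visible cursor and the character's CanSetMousePosition disabled.
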(event `self.ReceiveBeginPlay`
  (`parent.ReceiveBeginPlay`)
  (bind _returnvalue (`GameplayStatics.GetActorOfClass` "/Game/Beatriz/ReWork/BP_DayManager.BP_DayManager_C")))

(event `self.ReceiveTick`
  (params (DeltaSeconds :type "Float (single-precision)"))
  (bind __1 (`self.!1`))
  (bind _mesh (`self.Mesh`))
  (`parent.ReceiveTick` DeltaSeconds)
  (if (== (`/Game/Beatriz/ReWork/BP_DayManager.CurrentDay` (stale `self.ReceiveBeginPlay` _returnvalue)) 2)
    (`SceneComponent.SetVisibility` __1 true true)
    (set `self.IsSick?` true)
    (`SkeletalMeshComponent.PlayAnimation` _mesh "/Game/Beatriz/ReWork/Villagers/Sick_Idle.Sick_Idle" true)
    (else
      (`SceneComponent.SetVisibility` __1 false true)
      (set `self.IsSick?` false)
      (`SkeletalMeshComponent.PlayAnimation` _mesh "/Game/Beatriz/ReWork/Villagers/Man_Idle.Man_Idle" true))))

(event `self.Mesh.OnClicked`
  (params (TouchedComponent :type "PrimitiveComponent Object Reference") (ButtonPressed :type "Key Structure"))
  (bind _returnvalue (`GameplayStatics.GetPlayerController` 0))
  (if (`self.FirstClickTutorial`)
    (bind _returnvalue_2 (`|CreateWidget` "/Game/Widgets/Tutorial_WGT.Tutorial_WGT_C"))
    (`UserWidget.AddToViewport` _returnvalue_2 0)
    (`WidgetBlueprintLibrary.SetInputMode_UIOnlyEx` _returnvalue null)
    (set `PlayerController.bShowMouseCursor` true _returnvalue)
    (bind _asbp_first_person_character (cast `/Game/FirstPerson/Blueprints/BP_FirstPersonCharacter` (`GameplayStatics.GetPlayerCharacter` 0)))
    (set `/Game/FirstPerson/Blueprints/BP_FirstPersonCharacter.Can Set mouse position` false _asbp_first_person_character)))

(fn `UserConstructionScript`
  (`parent.UserConstructionScript`))