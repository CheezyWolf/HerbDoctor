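; Male villager Blueprint that shows as sick on day 0 and healthy on every other day.
; BeginPlay looks up BP_DayManager, whose CurrentDay is polled every Tick.
; Each Tick sets IsSick, shows or hides the component named "1", and calls PlayAnimation for a looping sick or normal idle, re-issuing it every frame rather than only when the day changes.
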(event `self.ReceiveBeginPlay`
  (`parent.ReceiveBeginPlay`)
  (bind _returnvalue (`GameplayStatics.GetActorOfClass` "/Game/Beatriz/ReWork/BP_DayManager.BP_DayManager_C")))

(event `self.ReceiveTick`
  (params (DeltaSeconds :type "Float (single-precision)"))
  (bind __1 (`self.!1`))
  (`parent.ReceiveTick` DeltaSeconds)
  (if (== (`/Game/Beatriz/ReWork/BP_DayManager.CurrentDay` (stale `self.ReceiveBeginPlay` _returnvalue)) 0)
    (`SceneComponent.SetVisibility` __1 true true)
    (set `self.IsSick?` true)
    (`SkeletalMeshComponent.PlayAnimation` (`self.Mesh`) "/Game/Beatriz/ReWork/Villagers/Sick_Idle.Sick_Idle" true)
    (else
      (`SceneComponent.SetVisibility` __1 false true)
      (set `self.IsSick?` false)
      (`SkeletalMeshComponent.PlayAnimation` (`self.Mesh`) "/Game/Beatriz/ReWork/Villagers/Man_IDle2.Man_IDle2" true))))

(fn `UserConstructionScript`
  (`parent.UserConstructionScript`))