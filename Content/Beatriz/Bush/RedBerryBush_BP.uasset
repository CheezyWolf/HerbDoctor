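; A red berry bush actor whose berry the player clicks to collect.
; BeginPlay enables click events and caches the first-person character.
; Clicking the berry plays a picking sound, adds a RedBerry to the player's inventory component, destroys the berry component and increments the character's BerriesCollected count.
; Both entering and leaving the sphere trigger hide the mouse cursor.
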(event `self.ReceiveBeginPlay`
  (set `PlayerController.bEnableClickEvents` true (`GameplayStatics.GetPlayerController` 0))
  (bind _asbp_first_person_character (cast `/Game/FirstPerson/Blueprints/BP_FirstPersonCharacter` (`GameplayStatics.GetPlayerCharacter` 0))))

(event `self.Berry.OnClicked`
  (params (TouchedComponent :type "PrimitiveComponent Object Reference") (ButtonPressed :type "Key Structure"))
  ;[1 1 1] Collect Berries
  (`KismetSystemLibrary.PrintString` "collected berry")
  (`GameplayStatics.PlaySound2D` "/Game/Maggie/Audio/HerbPickingSounds.HerbPickingSounds" 1.0 1.0 0.0 null null)
  (`/Game/Beatriz/ReWork/BP_InventoryComponent.AddItem` (`self.GetComponentByClass` (`GameplayStatics.GetPlayerCharacter` 0) "/Game/Beatriz/ReWork/BP_InventoryComponent.BP_InventoryComponent_C") "RedBerry" 1)
  (`ActorComponent.K2_DestroyComponent` (`self.Berry`))
  (`/Engine/EditorBlueprintResources/StandardMacros.IncrementInt` (`/Game/FirstPerson/Blueprints/BP_FirstPersonCharacter.Berries Collected` (stale `self.ReceiveBeginPlay` _asbp_first_person_character))))

(event `self.Sphere.OnComponentBeginOverlap`
  (params (OverlappedComponent :type "PrimitiveComponent Object Reference") (OtherActor :type "Actor Object Reference") (OtherComp :type "PrimitiveComponent Object Reference") (OtherBodyIndex :type Integer) (bFromSweep :type Boolean) (SweepResult :type "HitResult Structure (by ref)"))
  (set `PlayerController.bShowMouseCursor` false (`GameplayStatics.GetPlayerController` 0)))

(event `self.Sphere.OnComponentEndOverlap`
  (params (OverlappedComponent :type "PrimitiveComponent Object Reference") (OtherActor :type "Actor Object Reference") (OtherComp :type "PrimitiveComponent Object Reference") (OtherBodyIndex :type Integer))
  (set `PlayerController.bShowMouseCursor` false (`GameplayStatics.GetPlayerController` 0)))

(fn `UserConstructionScript`)