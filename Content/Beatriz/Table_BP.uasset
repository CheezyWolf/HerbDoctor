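; Crafting table actor that shows a crafting prompt and reveals the medicine once the player has crafted it.
; Box overlap adds a BeginCrafting_WGT to the viewport, throttled by a DoOnce that resets after one second, and end overlap removes it.
; The medicine mesh starts hidden, while Tick polls the first-person character's CraftedTheMeds flag through a short Delay to make it visible.
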(event `self.ReceiveBeginPlay`
  (`SceneComponent.SetVisibility` (`self.Meds_04`) false true))

(event `self.ReceiveTick`
  (params (DeltaSeconds :type "Float (single-precision)"))
  (`KismetSystemLibrary.Delay` 0.2)
  (`self.can medicine appear`))

(event `self.Box.OnComponentBeginOverlap`
  (params (OverlappedComponent :type "PrimitiveComponent Object Reference") (OtherActor :type "Actor Object Reference") (OtherComp :type "PrimitiveComponent Object Reference") (OtherBodyIndex :type Integer) (bFromSweep :type Boolean) (SweepResult :type "HitResult Structure (by ref)"))
  (`/Engine/EditorBlueprintResources/StandardMacros.DoOnce` false :!label _label
    (:`Completed`
      (bind _returnvalue (`|CreateWidget` "/Game/Widgets/BeginCrafting_WGT.BeginCrafting_WGT_C"))
      (bind _output_get (set `self.Widget crafting` _returnvalue))
      (`UserWidget.AddToViewport` _returnvalue 0)
      (`UserWidget.AddToViewport` _output_get 0)
      (`KismetSystemLibrary.Delay` 1.0)
      (goto _label :!via `Reset`))))

(event `self.Box.OnComponentEndOverlap`
  (params (OverlappedComponent :type "PrimitiveComponent Object Reference") (OtherActor :type "Actor Object Reference") (OtherComp :type "PrimitiveComponent Object Reference") (OtherBodyIndex :type Integer))
  (`Widget.RemoveFromParent` (stale `self.Box.OnComponentBeginOverlap` _returnvalue)))

(event `can medicine appear`
  (bind _asbp_first_person_character (cast `/Game/FirstPerson/Blueprints/BP_FirstPersonCharacter` (`GameplayStatics.GetPlayerCharacter` 0)))
  (if (`/Game/FirstPerson/Blueprints/BP_FirstPersonCharacter.Crafted the Meds` _asbp_first_person_character)
    (`SceneComponent.SetVisibility` (`self.medicine visibility`) true true)))

(fn `UserConstructionScript`)