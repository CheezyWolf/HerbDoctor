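; Fox AI pawn that wanders between four waypoints and plays a periodic fox call.
; From BeginPlay, a loop rolls randomly for a waypoint, re-rolling at each branch, and issues AIMoveTo.
; The loop continues two seconds after the move's immediate exec output, without waiting for arrival.
; Tick calls FoxNoise every frame, but its Delay spaces the non-spatial 2D sound about seven seconds apart.
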(event `self.ReceiveTick`
  (params (DeltaSeconds :type "Float (single-precision)"))
  (`self.Fox noise`))

(event `self.ReceiveBeginPlay`
  (`self.follow waypoint`)
  (`self.Fox noise`))

(event `Fox noise`
  (`KismetSystemLibrary.Delay` 7.0)
  (`GameplayStatics.PlaySound2D` "/Game/Animals/fox-calling-243999.fox-calling-243999" 1.0 1.0 0.0 null null))

(event `follow waypoint`
  (if (== (`KismetArrayLibrary.Array_Random` (`self.RandomWaypoint`)) 1) :!label _label
    (`|AIMoveTo` self (0.0 0.0 0.0) (`|GetArrayItem` (`self.waypoints`))
      (:`then`
        (`KismetSystemLibrary.Delay` 2.0)
        (goto _label)))
    (elif (== (`KismetArrayLibrary.Array_Random` (`self.RandomWaypoint`)) 2)
      ;[1 1 1] Comment
      (`|AIMoveTo` self (0.0 0.0 0.0) (`|GetArrayItem` (`self.waypoints`) 1)
        (:`then`
          (`KismetSystemLibrary.Delay` 2.0)
          (goto _label)))
      (elif (== (`KismetArrayLibrary.Array_Random` (`self.RandomWaypoint`)) 3)
        (`|AIMoveTo` self (0.0 0.0 0.0) (`|GetArrayItem` (`self.waypoints`) 2)
          (:`then`
            (`KismetSystemLibrary.Delay` 2.0)
            (goto _label)))
        (elif (== (`KismetArrayLibrary.Array_Random` (`self.RandomWaypoint`)) 4)
          (`|AIMoveTo` self (0.0 0.0 0.0) (`|GetArrayItem` (`self.waypoints`) 3)
            (:`then`
              (`KismetSystemLibrary.Delay` 2.0)
              (goto _label)))
          (else
            (goto _label)))))))

(fn `UserConstructionScript`)