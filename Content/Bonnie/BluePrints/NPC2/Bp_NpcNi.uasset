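; Bp_NpcNi is a clickable NPC that triggers the win screen once the player has crafted the first medicine part.
; An interact collision toggles a prompt widget, floating text and an animation value as the player enters and leaves, though any overlapping actor reveals the text.
; Clicking the mesh checks the first-person character's crafting flag, loops a dance, then shows YouWin_WGT with the cursor.
; The Tick-driven animation switch is an empty stub.
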(event `self.ReceiveBeginPlay`
  (bind _returnvalue (`|CreateWidget` "/Game/Bonnie/UIs/Npc_Interact.Npc_Interact_C"))
  (set `self.Interactprompt` _returnvalue)
  (set `PlayerController.bEnableClickEvents` true (`GameplayStatics.GetPlayerController` 0))
  (`SceneComponent.SetVisibility` (`self.TextRender`) false false))

(event `self.InteractCollision.OnComponentBeginOverlap`
  (params (OverlappedComponent :type "PrimitiveComponent Object Reference") (OtherActor :type "Actor Object Reference") (OtherComp :type "PrimitiveComponent Object Reference") (OtherBodyIndex :type Integer) (bFromSweep :type Boolean) (SweepResult :type "HitResult Structure (by ref)"))
  (`SceneComponent.SetVisibility` (`self.TextRender`) true false)
  ;[1 1 1] Interact Prompt Appears
  (if (== OtherActor (`GameplayStatics.GetPlayerCharacter` 0))
    (`UserWidget.AddToViewport` (`self.Interactprompt`) 0)
    (set `self.Animation Value ABP` 50.0)))

(event `self.InteractCollision.OnComponentEndOverlap`
  (params (OverlappedComponent :type "PrimitiveComponent Object Reference") (OtherActor :type "Actor Object Reference") (OtherComp :type "PrimitiveComponent Object Reference") (OtherBodyIndex :type Integer))
  ;[1 1 1] Interact Prompt Appears
  (if (== OtherActor (`GameplayStatics.GetPlayerCharacter` 0))
    (`Widget.RemoveFromParent` (`self.Interactprompt`))
    (`SceneComponent.SetVisibility` (`self.TextRender`) false false)
    (set `self.Animation Value ABP` 0.0)))

(event `self.NPCMeshOnlyfbx2.OnClicked`
  (params (TouchedComponent :type "PrimitiveComponent Object Reference") (ButtonPressed :type "Key Structure"))
  (bind _asbp_first_person_character (cast `/Game/FirstPerson/Blueprints/BP_FirstPersonCharacter` (`GameplayStatics.GetPlayerCharacter` 0)))
  (if (`/Game/FirstPerson/Blueprints/BP_FirstPersonCharacter.CraftedMedicine_Part1` _asbp_first_person_character)
    (`SkeletalMeshComponent.PlayAnimation` (`self.MaleKidModel1`) "/Game/Maggie/Animations/Dancing.Dancing" true)
    (`KismetSystemLibrary.Delay` 1.0)
    (bind _returnvalue (`|CreateWidget` "/Game/Widgets/YouWin_WGT.YouWin_WGT_C"))
    (`UserWidget.AddToViewport` _returnvalue 0)
    (set `PlayerController.bShowMouseCursor` true (`GameplayStatics.GetPlayerController` 0))
    (set `/Game/FirstPerson/Blueprints/BP_FirstPersonCharacter.Can Set mouse position` false _asbp_first_person_character)))

(event `self.ReceiveTick`
  (params (DeltaSeconds :type "Float (single-precision)"))
  (`KismetSystemLibrary.Delay` 1.0)
  (`self.Switch animation`))

(event `Switch animation`
  (if (`self.Idle`)
    _))

(fn `UserConstructionScript`)