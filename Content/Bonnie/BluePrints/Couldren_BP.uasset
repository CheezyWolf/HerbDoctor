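; Crafting cauldron actor that turns the player's first medicine part into Medicine_part2 when clicked.
; BeginPlay enables click events and caches the character; a click checks CraftedMedicinePart1, briefly shows a liquid plane, then spawns the item at PlaceToSpawnMedicine2.
; Overlap toggles an interact prompt and input, but E only re-casts the character.
; Prompt widget creation and an older berry-to-random-colour-medicine path are disconnected.
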(event `self.ReceiveBeginPlay`
  (set `PlayerController.bEnableClickEvents` true (`GameplayStatics.GetPlayerController` 0))
  ;[1 1 1] Checks if Player has picked Berries
  (bind _asbp_first_person_character (cast `/Game/FirstPerson/Blueprints/BP_FirstPersonCharacter` (`GameplayStatics.GetPlayerCharacter` 0) :!label _label)))

(event `self.UI_Collision.OnComponentBeginOverlap`
  (params (OverlappedComponent :type "PrimitiveComponent Object Reference") (OtherActor :type "Actor Object Reference") (OtherComp :type "PrimitiveComponent Object Reference") (OtherBodyIndex :type Integer) (bFromSweep :type Boolean) (SweepResult :type "HitResult Structure (by ref)"))
  ;[1 1 1] Press "E" To Interact UI
  (if (== OtherActor (`GameplayStatics.GetPlayerCharacter` 0))
    (`UserWidget.AddToViewport` (`self.InteractPrompt`) 0)
    ;[1 1 1] Press "E" liquid in couldren
    (`self.EnableInput` (`GameplayStatics.GetPlayerController` 0))))

(event `self.UI_Collision.OnComponentEndOverlap`
  (params (OverlappedComponent :type "PrimitiveComponent Object Reference") (OtherActor :type "Actor Object Reference") (OtherComp :type "PrimitiveComponent Object Reference") (OtherBodyIndex :type Integer))
  ;[1 1 1] Press "E" To Interact UI
  (if (== (`GameplayStatics.GetPlayerCharacter` 0) OtherActor)
    (`Widget.RemoveFromParent` (`self.InteractPrompt`))
    ;[1 1 1] Press "E" liquid in couldren
    (`self.DisableInput` (`GameplayStatics.GetPlayerController` 0))))

(event `Key|E`
  (params (Key :type "Key Structure"))
  ;[1 1 1] Checks if Player has picked Berries
  (:`Pressed`
    (goto _label)))

(event `self.Couldren_15.OnClicked`
  (params (TouchedComponent :type "PrimitiveComponent Object Reference") (ButtonPressed :type "Key Structure"))
  (bind _plane (`self.Plane`))
  (if (`/Game/FirstPerson/Blueprints/BP_FirstPersonCharacter.CraftedMedicine_Part1` (stale `self.ReceiveBeginPlay` _asbp_first_person_character))
    (`SceneComponent.SetVisibility` _plane true false)
    (`KismetSystemLibrary.PrintString` "crafting")
    (`KismetSystemLibrary.Delay` 1.5)
    (`SceneComponent.SetVisibility` _plane false false)
    (`|SpawnActorFromClass` "/Game/Beatriz/Medicine_part2.Medicine_part2_C" (`KismetMathLibrary.MakeTransform` (`SceneComponent.K2_GetComponentLocation` (`self.Place to spawn medicine 2`))) "Undefined" "MultiplyWithRoot" null null)))

(fn `UserConstructionScript`)