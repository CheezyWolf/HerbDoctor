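; BP_DiaComponent is an NPC dialogue component that shows data-table-driven conversation lines in a WB_Dialogue2 widget.
; DiaInteract creates the widget with the speaker name on first use, updates its text on later calls, and removes it once the end flag is set.
; Each row supplies the next row name, data table and end flag, so dialogue chains across tables.
; LeaveDialogue closes any open widget and clears the end flag.
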(event `/Game/Bonnie/BluePrints/Npc/NPC2/Bp_DiaInteract.LeaveDialogue`
  (`/Engine/EditorBlueprintResources/StandardMacros.IsValid` (`self.DialogueWidget`)
    (:`Is Valid`
      ;[1 1 1] Remove Dialogue
      (`Widget.RemoveFromParent` (`self.DialogueWidget`) :!label _label)
      (set `self.EndDia` false)
      (set `self.DialogueWidget` null))))

(event `/Game/Bonnie/BluePrints/Npc/NPC2/Bp_DiaInteract.DiaInteract`
  (params (Playerref :type "/Game/FirstPerson/Blueprints/BP_FirstPersonCharacter Object Reference"))
  (if (`self.EndDia`)
    (goto _label)
    (else
      (`/Engine/EditorBlueprintResources/StandardMacros.IsValid` (`self.DialogueWidget`)
        (:`Is Valid`
          ;[1 1 1] Next Dialgoue
          (bind _returnvalue (`|GetDataTableRow` (`self.Data Table`) (`self.Row Name`))
            (:`then`
              (bind (_dialogue _row _datatable _enddialogue) (break `/Game/Bonnie/BluePrints/Npc/NPC2/Dialogue_Structure` _returnvalue))
              (`/Game/Bonnie/BluePrints/Npc/NPC2/WB_Dialogue2.Update Dialogue` (`self.DialogueWidget`) _dialogue)
              (set `self.Row Name` _row)
              (set `self.Data Table` _datatable)
              (set `self.EndDia` _enddialogue))))
        (:`Is Not Valid`
          ;[1 1 1] Start Dialogue
          (bind _returnvalue_2 (`|GetDataTableRow` (`self.Data Table`) (`self.Row Name`))
            (:`then`
              (bind (_dialogue_2 _row_2 _datatable_2 _enddialogue_2) (break `/Game/Bonnie/BluePrints/Npc/NPC2/Dialogue_Structure` _returnvalue_2))
              (bind _returnvalue_3 (`|CreateWidget` "/Game/Bonnie/BluePrints/Npc/NPC2/WB_Dialogue2.WB_Dialogue2_C" null (`KismetTextLibrary.Conv_NameToText` (`self.name`)) _dialogue_2))
              (bind _output_get (set `self.DialogueWidget` _returnvalue_3))
              (`UserWidget.AddToViewport` _output_get 0)
              (set `self.Row Name` _row_2)
              (set `self.Data Table` _datatable_2)
              (set `self.EndDia` _enddialogue_2))))))))