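; NPC Blueprint for a character the player can cure with crafted medicine and hold a dialogue with.
; Clicking the mesh checks MedicineCrafted on BP_FirstPersonCharacter, then swaps the material to FlowerGreen and clears IsSick.
; The Talk event steps through the Dialogue array in a lazily created W_NPC_dialogue widget, removing it from the viewport once the lines run out.
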(event `self.NPCMeshOnlyfbx2.OnClicked`
  (params (TouchedComponent :type "PrimitiveComponent Object Reference") (ButtonPressed :type "Key Structure"))
  (bind _asbp_first_person_character (cast `/Game/FirstPerson/Blueprints/BP_FirstPersonCharacter` (`GameplayStatics.GetPlayerCharacter` 0)))
  (if (`/Game/FirstPerson/Blueprints/BP_FirstPersonCharacter.Medicine Crafted` _asbp_first_person_character)
    (`PrimitiveComponent.SetMaterial` (`self.NPCMeshOnlyfbx2`) 0 "/Game/Bonnie/Objects/Flowers/FlowerGreen.FlowerGreen")
    (set `self.Is sick` false)))

(event `/Game/Bonnie/BluePrints/Npc/BPI_Dialogue.Talk`
  ;[1 1 1] Dialogue
  (`/Engine/EditorBlueprintResources/StandardMacros.IncrementInt` (`self.Talkindex`)
    (:`  `
      (if (< (`self.Talkindex`) (`KismetArrayLibrary.Array_Length` (`self.Dialogue`)))
        (`self.UI`
          (:`then`
            _)
          (:`else`
            (bind _returnvalue (`|CreateWidget` "/Game/Bonnie/UIs/W_NPC_dialogue.W_NPC_dialogue_C" (`GameplayStatics.GetPlayerController` 0)))
            (bind _output_get (set `self.UI` _returnvalue))
            (`UserWidget.AddToViewport` _output_get 0)))
        (`TextBlock.SetText` (`/Game/Bonnie/UIs/W_NPC_dialogue.Talktext` (`self.UI`)) (`KismetTextLibrary.Conv_StringToText` (`|GetArrayItem` (`self.Dialogue`) (`self.Talkindex`))))
        (else
          (`Widget.RemoveFromParent` (`self.UI`)))))))

(fn `UserConstructionScript`)