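; Test cauldron actor for crafting medicine.
; Overlapping its collision shows an interact widget and enables input, so E spawns a Medicine_BP at a hardcoded location after a delay, randomly tinted through a dynamic material.
; Separately, clicking the cauldron mesh checks the player's MedicinePart2, briefly shows the cylinder during a delay, then spawns Medicine_part3 at a marker component.
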(event `self.ReceiveBeginPlay`
  (bind _returnvalue (`|CreateWidget` "/Game/Bonnie/UIs/Caul_Interact.Caul_Interact_C"))
  (set `self.Interact` _returnvalue)
  (bind _asbp_first_person_character (cast `/Game/FirstPerson/Blueprints/BP_FirstPersonCharacter` (`GameplayStatics.GetPlayerCharacter` 0))))

(event `self.Collision.OnComponentBeginOverlap`
  (params (OverlappedComponent :type "PrimitiveComponent Object Reference") (OtherActor :type "Actor Object Reference") (OtherComp :type "PrimitiveComponent Object Reference") (OtherBodyIndex :type Integer) (bFromSweep :type Boolean) (SweepResult :type "HitResult Structure (by ref)"))
  ;[1 1 1] Press "E" To Interact UI
  (if (== OtherActor (`GameplayStatics.GetPlayerCharacter` 0))
    (`UserWidget.AddToViewport` (`self.Interact`) 0)
    (`self.EnableInput` (`GameplayStatics.GetPlayerController` 0))))

(event `self.Collision.OnComponentEndOverlap`
  (params (OverlappedComponent :type "PrimitiveComponent Object Reference") (OtherActor :type "Actor Object Reference") (OtherComp :type "PrimitiveComponent Object Reference") (OtherBodyIndex :type Integer))
  ;[1 1 1] Press "E" To Interact UI
  (if (== (`GameplayStatics.GetPlayerCharacter` 0) OtherActor)
    (`Widget.RemoveFromParent` (`self.Interact`))
    (`self.DisableInput` (`GameplayStatics.GetPlayerController` 0))))

(event `Key|E`
  (params (Key :type "Key Structure"))
  (:`Pressed`
    (`KismetSystemLibrary.Delay` 1.0)
    (bind _returnvalue (`|SpawnActorFromClass` "/Game/Bonnie/BluePrints/Medicine_BP.Medicine_BP_C" (`KismetMathLibrary.MakeTransform` (-584.0 -434.0 0.0)) "Undefined" "MultiplyWithRoot" null null))
    (bind _returnvalue_2 (`PrimitiveComponent.CreateDynamicMaterialInstance` (`/Game/Bonnie/BluePrints/Medicine_BP.Meds_04` _returnvalue) 2 "/Game/Bonnie/Objects/Medicine/M_DynamicColor.M_DynamicColor" "None"))
    (`MaterialInstanceDynamic.SetVectorParameterValue` _returnvalue_2 "MedChangeColor" (make `LinearColor` (`KismetMathLibrary.RandomFloat`) (`KismetMathLibrary.RandomFloat`) (`KismetMathLibrary.RandomFloat`) 1.0))))

(event `self.Couldren_15.OnClicked`
  (params (TouchedComponent :type "PrimitiveComponent Object Reference") (ButtonPressed :type "Key Structure"))
  (if (`/Game/FirstPerson/Blueprints/BP_FirstPersonCharacter.Medicine part 2` (stale `self.ReceiveBeginPlay` _asbp_first_person_character))
    (`SceneComponent.SetVisibility` (`self.Cylinder`) true false)
    (`KismetSystemLibrary.PrintString` "crafting medicine")
    (`KismetSystemLibrary.Delay` 1.5)
    (`|SpawnActorFromClass` "/Game/Beatriz/Medicine_part3.Medicine_part3_C" (`KismetMathLibrary.MakeTransform` (`SceneComponent.K2_GetComponentLocation` (`self.place to spawn medicine 3`))) "Undefined" "MultiplyWithRoot" null null)
    (`SceneComponent.SetVisibility` (`self.Cylinder`) false false)))

(fn `UserConstructionScript`)