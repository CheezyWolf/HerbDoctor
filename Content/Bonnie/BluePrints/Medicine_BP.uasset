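; Medicine pickup actor that the player collects with E, setting MedicineCrafted on BP_FirstPersonCharacter.
; Box_Collision overlap shows or hides the Collect_Interact prompt and toggles the actor's input for the player.
; Pressing E destroys only the Meds04 component, then hides the mouse cursor and sets CanSetMousePosition on the character.
; A disconnected YouWin_WGT branch never runs.
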(event `self.ReceiveBeginPlay`
  (bind _returnvalue (`|CreateWidget` "/Game/Bonnie/UIs/Collect_Interact.Collect_Interact_C"))
  (set `self.CollectPrompt` _returnvalue))

(event `self.Box_Collision.OnComponentBeginOverlap`
  (params (OverlappedComponent :type "PrimitiveComponent Object Reference") (OtherActor :type "Actor Object Reference") (OtherComp :type "PrimitiveComponent Object Reference") (OtherBodyIndex :type Integer) (bFromSweep :type Boolean) (SweepResult :type "HitResult Structure (by ref)"))
  ;[1 1 1] Interact prompt
  (if (== OtherActor (`GameplayStatics.GetPlayerCharacter` 0))
    (`UserWidget.AddToViewport` (`self.CollectPrompt`) 0)
    (`self.EnableInput` (`GameplayStatics.GetPlayerController` 0))))

(event `self.Box_Collision.OnComponentEndOverlap`
  (params (OverlappedComponent :type "PrimitiveComponent Object Reference") (OtherActor :type "Actor Object Reference") (OtherComp :type "PrimitiveComponent Object Reference") (OtherBodyIndex :type Integer))
  ;[1 1 1] Interact prompt
  (if (== (`GameplayStatics.GetPlayerCharacter` 0) OtherActor)
    (`Widget.RemoveFromParent` (`self.CollectPrompt`))
    (`self.DisableInput` (`GameplayStatics.GetPlayerController` 0))))

(event `Key|E`
  (params (Key :type "Key Structure"))
  (:`Pressed`
    (`ActorComponent.K2_DestroyComponent` (`self.Meds_04`))
    (bind _asbp_first_person_character (cast `/Game/FirstPerson/Blueprints/BP_FirstPersonCharacter` (`GameplayStatics.GetPlayerCharacter` 0)))
    (set `/Game/FirstPerson/Blueprints/BP_FirstPersonCharacter.Medicine Crafted` true _asbp_first_person_character)
    (set `PlayerController.bShowMouseCursor` false (`GameplayStatics.GetPlayerController` 0))
    (set `/Game/FirstPerson/Blueprints/BP_FirstPersonCharacter.Can Set mouse position` true _asbp_first_person_character)))

(fn `UserConstructionScript`)