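; PickableBush_BP is a bush actor that shows an interaction prompt when the player is near; it contains no picking logic itself.
; On BeginPlay it creates a Bush_Interact widget and stores it as InteractPrompt.
; Box_Collision overlap events add that widget to the viewport when the first player's character enters and remove it when that character leaves.
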(event `self.ReceiveBeginPlay`
  (bind _returnvalue (`|CreateWidget` "/Game/Bonnie/UIs/Bush_Interact.Bush_Interact_C"))
  (set `self.InteractPrompt` _returnvalue))

(event `self.Box_Collision.OnComponentBeginOverlap`
  (params (OverlappedComponent :type "PrimitiveComponent Object Reference") (OtherActor :type "Actor Object Reference") (OtherComp :type "PrimitiveComponent Object Reference") (OtherBodyIndex :type Integer) (bFromSweep :type Boolean) (SweepResult :type "HitResult Structure (by ref)"))
  ;[1 1 1] Interact Prompt
  (if (== OtherActor (`GameplayStatics.GetPlayerCharacter` 0))
    (`UserWidget.AddToViewport` (`self.InteractPrompt`) 0)))

(event `self.Box_Collision.OnComponentEndOverlap`
  (params (OverlappedComponent :type "PrimitiveComponent Object Reference") (OtherActor :type "Actor Object Reference") (OtherComp :type "PrimitiveComponent Object Reference") (OtherBodyIndex :type Integer))
  ;[1 1 1] Interact Prompt
  (if (== (`GameplayStatics.GetPlayerCharacter` 0) OtherActor)
    (`Widget.RemoveFromParent` (`self.InteractPrompt`))))

(fn `UserConstructionScript`)