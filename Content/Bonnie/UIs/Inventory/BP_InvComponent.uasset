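; Inventory component with nine slots, shown through a Widget_Inv that Tab toggles on screen.
; Left click sphere-traces around the player's feet for a BP_Item, stacks it up to 64 or fills an empty slot, then refreshes the widget and destroys the item.
; It also forwards berries and roots to BP_InventoryComponent by the slot's name.
; The mortar-and-pestle flag branch repeats the Root check, so it never runs.
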(event `self.ReceiveBeginPlay`
  (bind _returnvalue (`|CreateWidget` "/Game/Bonnie/UIs/Inventory/Widget_Inv.Widget_Inv_C"))
  (set `self.InvWidget` _returnvalue)
  (`KismetArrayLibrary.Array_Resize` (`self.Items`) 9)
  (`/Game/Bonnie/UIs/Inventory/Widget_Inv.Load Inventory` (`self.InvWidget`) self))

(event `Key|Tab`
  (params (Key :type "Key Structure"))
  (bind _invwidget (`self.InvWidget`))
  ;[1 1 1] Show/Hide Inventory
  (:`Pressed`
    (if (`Widget.IsVisible` (`self.InvWidget`))
      (`Widget.RemoveFromParent` _invwidget)
      (else
        (`UserWidget.AddToViewport` _invwidget 0)))))

(event `Key|LeftMouseButton`
  (params (Key :type "Key Structure"))
  (bind _returnvalue (`Actor.GetComponentByClass` (`GameplayStatics.GetPlayerCharacter` 0) "/Game/Beatriz/ReWork/BP_InventoryComponent.BP_InventoryComponent_C"))
  (bind _returnvalue_2 (- (`Actor.K2_GetActorLocation` (`GameplayStatics.GetPlayerCharacter` 0)) (0.0 0.0 65.0)))
  ;[1 1 1] Add to Inventory
  (:`Pressed`
    (bind _outhit (`KismetSystemLibrary.SphereTraceSingle` :`Start` _returnvalue_2 :`End` _returnvalue_2 :`Radius` 140.0 :`TraceChannel` "TraceTypeQuery1" :`DrawDebugType` "ForDuration"))
    (bind _asbp_item (cast `/Game/Bonnie/UIs/Inventory/BP_Item` (`.HitActor` (`GameplayStatics.BreakHitResult` _outhit))))
    (for (_array_element _array_index) (`self.Items`)
      (`/Engine/EditorBlueprintResources/StandardMacros.IsValid` _asbp_item
        (:`Is Valid`
          (bind (_name _stackable _quantity) (break `/Game/Bonnie/UIs/Inventory/S_ItemStructure` _array_element))
          (bind (_name_2 _stackable_2 _quantity_2) (break `/Game/Bonnie/UIs/Inventory/S_ItemStructure` (`/Game/Bonnie/UIs/Inventory/BP_Item.Item` _asbp_item)))
          (bind _returnvalue_3 (+ _quantity _quantity_2))
          (if (and (`KismetTextLibrary.EqualEqual_TextText` _name _name_2) _stackable_2 (<= _returnvalue_3 64))
            (bind (_item_name _item_stackable _item_quantity _item_thumbnail _item_mesh) (break `/Game/Bonnie/UIs/Inventory/S_ItemStructure` (`/Game/Bonnie/UIs/Inventory/BP_Item.Item` _asbp_item)))
            (`KismetArrayLibrary.Array_Set` (`self.Items`) _array_index (make `/Game/Bonnie/UIs/Inventory/S_ItemStructure` _item_name _item_stackable _returnvalue_3 _item_thumbnail _item_mesh))
            (`/Game/Bonnie/UIs/Inventory/Widget_Inv.Load Inventory` (`self.InvWidget`) self :!label _label)
            (`|ExecutionSequence`
              (:`then_0`
                (`Actor.K2_DestroyActor` _asbp_item))
              (:`then_1`
                (bind _returnvalue_4 (`KismetTextLibrary.Conv_TextToString` _name))
                (if (`KismetStringLibrary.EqualEqual_StrStr` _returnvalue_4 "RedBerry")
                  (`/Game/Beatriz/ReWork/BP_InventoryComponent.AddItem` _returnvalue "RedBerry" 1)
                  (elif (`KismetStringLibrary.EqualEqual_StrStr` _returnvalue_4 "BlueBerry")
                    (`/Game/Beatriz/ReWork/BP_InventoryComponent.AddItem` _returnvalue "BlueBerry" 1)
                    (elif (`KismetStringLibrary.EqualEqual_StrStr` _returnvalue_4 "Root")
                      (`/Game/Beatriz/ReWork/BP_InventoryComponent.AddItem` _returnvalue "Root" 1)
                      (elif (`KismetStringLibrary.EqualEqual_StrStr` _returnvalue_4 "Root")
                        (bind _asbp_first_person_character (cast `/Game/FirstPerson/Blueprints/BP_FirstPersonCharacter` (`GameplayStatics.GetPlayerCharacter` 0)))
                        (set `/Game/FirstPerson/Blueprints/BP_FirstPersonCharacter.Have Mortat and Pestle?` true _asbp_first_person_character)))))))
            (elif (== _quantity 0)
              (`KismetArrayLibrary.Array_Set` (`self.Items`) _array_index (`/Game/Bonnie/UIs/Inventory/BP_Item.Item` _asbp_item))
              (goto _label))))))))