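; AC_HeldComponent is a component that tracks how long a key is held and shows it on a mini-game progress bar.
; BeginPlay creates and stores the MiniGame_Widget without adding it to the screen.
; The CheckKeyHold event, not called within this graph, reads the key's down time from the player controller and sets HeldBar to its fraction of MaxHold.
; It removes the widget only when hold time exactly equals MaxHold.
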(event `self.ReceiveBeginPlay`
  (bind _returnvalue (`|CreateWidget` "/Game/MiniGame_Widget.MiniGame_Widget_C"))
  (set `self.Held Key Widget` _returnvalue))

(event `CheckKeyHold`
  (set `self.Holding Time` (`PlayerController.GetInputKeyTimeDown` (`GameplayStatics.GetPlayerController` 0) (`self.Key Pressed`)))
  (`ProgressBar.SetPercent` (`/Game/MiniGame_Widget.HeldBar` (`self.Held Key Widget`)) (/ (`self.Holding Time`) (`self.Max Hold`)))
  (if (== (`self.Holding Time`) (`self.Max Hold`))
    (`Widget.RemoveFromParent` (`self.Held Key Widget`))))